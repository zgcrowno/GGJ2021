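; First-person player character, named as unused, with movement, footstep audio, object highlighting and interaction.
; Each tick it sets velocity from input, marks traced "Highlightable" components through custom depth stencil, and animates a ripple radius that restarts while moving.
; A dynamic post-process material is added to the camera at BeginPlay, and a timeline paced by forward input fires footstep sounds.
; Interact messages the first overlapping BPi_Interactable actor, independent of the highlight trace.
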(event EventBeginPlay
  (Utilities|FlowControl|Sequence
    (:then_0
      (Utilities|Array|AddUnique (Variables|Default|GetSenses) 0)
      (bind _returnvalue (Rendering|Material|CreateDynamicMaterialInstance "/Game/Materials/M_Highlight_Inst.M_Highlight_Inst" "None" :!class /Script/Engine.KismetMaterialLibrary))
      (bind _output_get (Variables|Default|SetRippleMaterialInst _returnvalue))
      (Utilities|Array|Add (Utilities|Struct|BreakWeightedBlendables (Utilities|Struct|BreakPostProcessSettings (Variables|/Script/Engine.CameraComponent|GetPostProcessSettings (Variables|Default|GetCamera)))) (Utilities|Struct|MakeWeightedBlendable 1.0 _output_get)))
    (:then_1
      (Components|Timeline|SetPlayRate (Variables|Default|GetFootStepTimeline) 0.0)
      (Timeline|FootStepTimeline Play
        (:Footsteps%20Event
          (Audio|SpawnSoundatLocation "/Game/Audio/SFX/SoundCues/FootSteps_SFX_Cue.FootSteps_SFX_Cue" (Transformation|GetWorldLocation (Variables|Default|GetFeetLocation)) "0, 0, 0" 1.0 1.0 0.0 0 0))))))

(event Collision|EventActorBeginOverlap
  (params (OtherActor :type Actor%20Object%20Reference)))

(event EventTick
  (params (DeltaSeconds :type Float%20%28single-precision%29))
  (CallFunction|Move)
  (CallFunction|Highlight)
  (CallFunction|Ripple))

(event Input|ActionEvents|InputActionInteract
  (params (Key :type Key%20Structure :default "None"))
  (:Pressed
    (bind _array_element (Utilities|Array|ForEachLoopwithBreak (Collision|GetOverlappingActors (Variables|Collision|GetCapsuleComponent) 0 :!class /Script/Engine.PrimitiveComponent) :!label _label)
      (:LoopBody
        (if (Utilities|DoesObjectImplementInterface _array_element "/Game/Blueprints/BPi_Interactable.BPi_Interactable_C")
          (Class|BPiInteractable|Interaction(Message) _array_element)
          (goto _label Break))))))

(event Input|AxisEvents|InputAxisMoveForward
  (params (AxisValue :type Float%20%28single-precision%29))
  (Components|Timeline|SetPlayRate (Variables|Default|GetFootStepTimeline) (* AxisValue 1.5)))

(event Input|MouseEvents|MouseX
  (params (AxisValue :type Float%20%28single-precision%29))
  (Pawn|Input|AddControllerYawInput AxisValue))

(event Input|MouseEvents|MouseY
  (params (AxisValue :type Float%20%28single-precision%29))
  (bind _result (Math|Float|NegateFloat AxisValue)
    (:%20%20
      (Pawn|Input|AddControllerPitchInput _result))))

(fn ConstructionScript)

(fn Move
  (bind _returnvalue (Utilities|Time|GetWorldDeltaSeconds))
  (bind _movespeed (Variables|Default|GetMoveSpeed))
  (bind _output_get (LocalVariables|SetMovementVec (+ (+ (* (Transformation|GetActorForwardVector) (* (* (Input|AxisValues|GetMoveForward) _movespeed) _returnvalue)) (* (Transformation|GetActorRightVector) (* _returnvalue (* _movespeed (Input|AxisValues|GetMoveRight))))) (Math|Vector|MakeVector 0.0 0.0 (.Z (Math|Vector|BreakVector (Variables|/Script/Engine.MovementComponent|GetVelocity (Variables|Character|GetCharacterMovement))))))))
  (bind _output_get_2 (Variables|/Script/Engine.MovementComponent|SetVelocity (Variables|Character|GetCharacterMovement) _output_get))
  (if (not (Math|Vector|Equal(Vector) _output_get_2 "0, 0, 0" 0.0001))
    (if (<= (Variables|Default|GetRippleLifetime) 0.0)
      (Variables|Default|SetRippleLifetime (Variables|Default|GetMaxRippleLifetime)))))

(fn Highlight
  (bind _camera (Variables|Default|GetCamera))
  (bind _returnvalue (Transformation|GetWorldLocation _camera))
  (if (Utilities|IsValid (Variables|Default|GetHighlightedObject))
    (Rendering|SetCustomDepthStencilValue (Variables|Default|GetHighlightedObject) 0))
  (bind (_outhit _returnvalue_2) (Collision|LineTraceByChannel _returnvalue (+ _returnvalue (* (Math|Vector|GetForwardVector _camera) (Variables|Default|GetInteractDistance))) "TraceTypeQuery1" false 0 "ForOneFrame"))
  (if _returnvalue_2
    (if (Components|ComponentHasTag (.HitComponent (Collision|BreakHitResult _outhit)) "Highlightable")
      (bind _output_get (Variables|Default|SetHighlightedObject (.HitComponent (Collision|BreakHitResult _outhit))))
      (Rendering|SetCustomDepthStencilValue _output_get 1))))

(fn Ripple
  (if (> (Variables|Default|GetRippleLifetime) 0.0)
    (Rendering|Material|SetScalarParameterValue 0 "Radius" (- 1.0 (/ (Variables|Default|GetRippleLifetime) (Variables|Default|GetMaxRippleLifetime))) :!class /Script/Engine.KismetMaterialLibrary)
    (Variables|Default|SetRippleLifetime (- (Variables|Default|GetRippleLifetime) (Utilities|Time|GetWorldDeltaSeconds)))))