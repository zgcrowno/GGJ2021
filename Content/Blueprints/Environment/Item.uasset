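; Pickup item that a pawn can collect through an interaction and that carries a key value.
; On interaction it sends itself to the pawn and, if accepted, teleports its Cone component to a deactivated location instead of destroying the actor.
; Pawn overlap shows an ItemPickup prompt widget, and leaving removes widgets of that class.
; GiveKeyValue exposes the key, while CheckForKey returns fixed enum values and PickUp is empty.
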(event Collision|EventActorBeginOverlap
  (params (OtherActor :type Actor%20Object%20Reference))
  (Utilities|Casting|CastToPawn OtherActor)
  (bind _returnvalue (UserInterface|CreateWidget "/Game/Blueprints/Widgets/itemPickup.itemPickup_C"))
  (UserInterface|Viewport|AddtoViewport _returnvalue 0))

(event Collision|EventActorEndOverlap
  (params (OtherActor :type Actor%20Object%20Reference))
  (Utilities|Casting|CastToPawn OtherActor)
  (bind _foundwidgets (Widget|GetAllWidgetsOfClass "/Game/Blueprints/Widgets/itemPickup.itemPickup_C" true))
  (Widget|RemovefromParent _foundwidgets))

(event EventInteraction
  (params (Interactor :type Actor%20Object%20Reference))
  (bind _aspawn (Utilities|Casting|CastToPawn Interactor))
  (bind _waspickedup (Class|BPiInteractable|PickUp(Message) _aspawn self))
  (if _waspickedup
    (Transformation|SetWorldLocation (Variables|Default|GetCone) (Variables|Default|GetdeactivatedLocation) false false)))

(fn ConstructionScript)

(fn GiveKeyValue
  (return (Variables|Default|GetKeyValue)))

(fn CheckforKey
  (return "NewEnumerator3" "NewEnumerator3"))

(fn PickUp
  (params (theItem :type Item%20Object%20Reference)))