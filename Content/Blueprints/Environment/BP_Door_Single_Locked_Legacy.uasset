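; Single locked door that pawns open or close through an interaction event when one of their two key slots matches UnlockedBy.
; A match, checked through message calls on the pawn, consumes the key, destroys all text components and animates rotation with MoveComponentTo.
; No unlocked state is stored, so every toggle repeats the key check.
; Overlap shows the prompt on both sides, and a failed check briefly toggles the locked text using a timer.
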(event Collision|EventActorBeginOverlap
  (params (OtherActor :type Actor%20Object%20Reference))
  (bind _text_front (Variables|Default|GetText_front))
  (bind _text_back (Variables|Default|GetText_back))
  ;[1 1 1] Toggles the prompt when the user is in range
  (Utilities|Casting|CastToPawn OtherActor)
  (if (Utilities|IsValid _text_front)
    (Rendering|SetVisibility _text_front true false))
  (if (Utilities|IsValid _text_back)
    (Rendering|SetVisibility _text_back true false)))

(event EventBeginPlay)

(event Collision|EventActorEndOverlap
  (params (OtherActor :type Actor%20Object%20Reference))
  (bind _text_front (Variables|Default|GetText_front))
  (bind _text_back (Variables|Default|GetText_back))
  ;[1 1 1] Toggles the prompt when the user is in range
  (Utilities|Casting|CastToPawn OtherActor)
  (if (Utilities|IsValid _text_front)
    (Rendering|SetVisibility _text_front false false))
  (if (Utilities|IsValid _text_back)
    (Rendering|SetVisibility _text_back false false)))

(event EventInteraction
  (params (Interactor :type Actor%20Object%20Reference))
  (bind _unlockedby (Variables|Default|GetunlockedBy))
  (bind _livingroom_door_abagailrobb (Variables|Default|GetLivingRoom_Door_AbagailRobb))
  (bind _livingroom_door_abagailrobb_2 (Variables|Default|GetLivingRoom_Door_AbagailRobb))
  (bind _aspawn (Utilities|Casting|CastToPawn Interactor))
  (bind (_key_value_1 _key_value_2) (Class|BPiInteractable|CheckforKey(Message) _aspawn))
  (if (or (Utilities|Enum|Equal(Enum) _key_value_1 _unlockedby) (Utilities|Enum|Equal(Enum) _key_value_2 _unlockedby))
    (Class|BPiInteractable|DestroyKey(Message) _aspawn _unlockedby)
    (Components|DestroyComponent (Variables|Default|GetLocked_front))
    (Components|DestroyComponent (Variables|Default|GetLocked_back))
    (Components|DestroyComponent (Variables|Default|GetText_front))
    (Components|DestroyComponent (Variables|Default|GetText_back))
    (if (Variables|Default|GetisOpen)
      ;[1 1 1] Close Door
      (Components|MoveComponentTo _livingroom_door_abagailrobb_2 (Variables|/Script/Engine.SceneComponent|GetRelativeLocation _livingroom_door_abagailrobb_2) (Variables|Default|GetclosedRotation) false false 1.0 false)
      (Variables|Default|SetisOpen false)
      (else
        ;[1 1 1] Open Door
        (Components|MoveComponentTo _livingroom_door_abagailrobb (Variables|/Script/Engine.SceneComponent|GetRelativeLocation _livingroom_door_abagailrobb) (Variables|Default|GetopenRotation) false false 1.0 false)
        (Variables|Default|SetisOpen true)))
    (else
      (CallFunction|ToggleLockedDisplay)
      (Utilities|Time|SetTimerbyFunctionName 0 "ToggleLockedDisplay" 2.0))))

(fn ConstructionScript
  (bind _text_front (Variables|Default|GetText_front))
  (bind _presse (Variables|Default|GetpressE))
  (bind _text_back (Variables|Default|GetText_back))
  (bind _locked_front (Variables|Default|GetLocked_front))
  (bind _lockedbuddyboy (Variables|Default|GetlockedBuddyBoy))
  (bind _locked_back (Variables|Default|GetLocked_back))
  ;[1 1 1] Sets prompt text and hides it
  (Rendering|Components|TextRender|SetText _text_front _presse)
  (Rendering|Components|TextRender|SetText _text_back _presse)
  (Rendering|SetVisibility _text_front false false)
  (Rendering|SetVisibility _text_back false false)
  ;[1 1 1] Sets Locked text and hides it
  (Rendering|Components|TextRender|SetText _locked_front _lockedbuddyboy)
  (Rendering|SetVisibility _locked_front false false)
  (Rendering|Components|TextRender|SetText _locked_back _lockedbuddyboy)
  (Rendering|SetVisibility _locked_back false false))

(fn ToggleLockedDisplay
  (bind _locked_back (Variables|Default|GetLocked_back))
  (bind _locked_front (Variables|Default|GetLocked_front))
  (if (Utilities|IsValid _locked_back)
    (Rendering|ToggleVisibility _locked_back false))
  (if (Utilities|IsValid _locked_front)
    (Rendering|ToggleVisibility _locked_front false)))

(fn CheckforKey
  (return "NewEnumerator3" "NewEnumerator3"))

(fn PickUp
  (params (theItem :type Item%20Object%20Reference))
  (return false))