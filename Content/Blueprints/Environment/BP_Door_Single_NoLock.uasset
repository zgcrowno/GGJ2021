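; Single unlocked door Blueprint that a Pawn can swing open or closed through its Interaction event.
; Each interaction flips IsOpen and rotates the door mesh between open and closed rotations with MoveComponentTo.
; Actor overlap shows and hides front and back prompt texts, which the construction script fills and hides initially.
; Locked text, ShowLocked and an always-false CheckForKey exist but play no part in the interaction flow.
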(event Collision|EventActorBeginOverlap
  (params (OtherActor :type Actor%20Object%20Reference))
  (Utilities|Casting|CastToPawn OtherActor)
  (Rendering|SetVisibility (Variables|Default|GetText_front) true false)
  (Rendering|SetVisibility (Variables|Default|GetText_back) true false))

(event EventBeginPlay)

(event Collision|EventActorEndOverlap
  (params (OtherActor :type Actor%20Object%20Reference))
  (Utilities|Casting|CastToPawn OtherActor)
  (Rendering|SetVisibility (Variables|Default|GetText_front) false false)
  (Rendering|SetVisibility (Variables|Default|GetText_back) false false))

(event EventInteraction
  (params (Interactor :type Actor%20Object%20Reference))
  (bind _livingroom_door_abagailrobb (Variables|Default|GetLivingRoom_Door_AbagailRobb))
  (bind _livingroom_door_abagailrobb_2 (Variables|Default|GetLivingRoom_Door_AbagailRobb))
  (Utilities|Casting|CastToPawn Interactor)
  (if (Variables|Default|GetisOpen)
    ;[1 1 1] Close Door
    (Components|MoveComponentTo _livingroom_door_abagailrobb_2 (Variables|/Script/Engine.SceneComponent|GetRelativeLocation _livingroom_door_abagailrobb_2) (Variables|Default|GetclosedRotation) false false 1.0 false)
    (Variables|Default|SetisOpen false)
    (else
      ;[1 1 1] Open Door
      (Components|MoveComponentTo _livingroom_door_abagailrobb (Variables|/Script/Engine.SceneComponent|GetRelativeLocation _livingroom_door_abagailrobb) (Variables|Default|GetopenRotation) false false 1.0 false)
      (Variables|Default|SetisOpen true))))

(fn ConstructionScript
  (bind _text_front (Variables|Default|GetText_front))
  (bind _presse (Variables|Default|GetpressE))
  (bind _text_back (Variables|Default|GetText_back))
  (bind _locked_front (Variables|Default|GetLocked_front))
  (bind _lockedbuddyboy (Variables|Default|GetlockedBuddyBoy))
  (bind _locked_back (Variables|Default|GetLocked_back))
  ;[1 1 1] Sets prompt text and hides it
  (Rendering|Components|TextRender|SetText _text_front _presse)
  (Rendering|Components|TextRender|SetText _text_back _presse)
  (Rendering|SetVisibility _text_front false false)
  (Rendering|SetVisibility _text_back false false)
  ;[1 1 1] Sets Locked text and hides it
  (Rendering|Components|TextRender|SetText _locked_front _lockedbuddyboy)
  (Rendering|SetVisibility _locked_front false false)
  (Rendering|Components|TextRender|SetText _locked_back _lockedbuddyboy)
  (Rendering|SetVisibility _locked_back false false))

(fn ShowLocked
  (Rendering|ToggleVisibility (Variables|Default|GetLocked_back) false)
  (Rendering|ToggleVisibility (Variables|Default|GetLocked_front) false))

(fn CheckforKey
  (return false))