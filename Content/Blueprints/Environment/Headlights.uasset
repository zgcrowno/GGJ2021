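; Headlights actor that drives forward every frame and triggers a screen transition into another level once its X position drops below a threshold.
; Tick runs chained countdown timers that ramp MPC_EyeAdjust Intensity up, then back down, then hold before opening the "Test" level.
; The player camera's post-process blendables receive an eye-adjust material, which is swapped for a headlight-transition material at peak intensity.
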(event EventBeginPlay
  (bind _returnvalue (Actor|GetActorOfClass "/Game/Blueprints/BP_Player.BP_Player_C"))
  (Variables|Default|SetPlayerCamera (Actor|GetComponentbyClass _returnvalue "/Script/Engine.CameraComponent"))
  (bind _returnvalue_2 (Rendering|Material|CreateDynamicMaterialInstance "/Game/Materials/M_HeadlightTransition_Inst.M_HeadlightTransition_Inst" "None" :!class /Script/Engine.KismetMaterialLibrary))
  (Variables|Default|SetHeadlightTransitionInst _returnvalue_2)
  (bind _returnvalue_3 (Rendering|Material|CreateDynamicMaterialInstance "/Game/Materials/M_EyeAdjust.M_EyeAdjust" "None" :!class /Script/Engine.KismetMaterialLibrary))
  (Variables|Default|SetEyeAdjustInst _returnvalue_3))

(event Collision|EventActorBeginOverlap
  (params (OtherActor :type Actor%20Object%20Reference)))

(event EventTick
  (params (DeltaSeconds :type Float%20%28single-precision%29))
  (Transformation|SetActorLocation (+ (Transformation|GetActorLocation) (* (Transformation|GetActorForwardVector) (Variables|Default|GetMoveSpeed))) false false)
  (if (< (.X (Math|Vector|BreakVector (Transformation|GetActorLocation))) (Variables|Default|GetLevelTransitionDistance))
    (if (and (and (<= (Variables|Default|GetBlackToWhiteTime) 0.0) (<= (Variables|Default|GetWhiteToBlackTime) 0.0)) (<= (Variables|Default|GetTransitionTime) 0.0))
      (Variables|Default|SetBlackToWhiteTime (Variables|Default|GetMaxBlackToWhiteTime))
      (Utilities|Array|Add (Utilities|Struct|BreakWeightedBlendables (Utilities|Struct|BreakPostProcessSettings (Variables|/Script/Engine.CameraComponent|GetPostProcessSettings (Variables|Default|GetPlayerCamera)))) (Utilities|Struct|MakeWeightedBlendable 1.0 (Variables|Default|GetEyeAdjustInst)))
      (elif (> (Variables|Default|GetBlackToWhiteTime) 0.0)
        (Rendering|Material|SetScalarParameterValue "/Game/Materials/MPC_EyeAdjust.MPC_EyeAdjust" "Intensity" (- 1.0 (/ (Variables|Default|GetBlackToWhiteTime) (Variables|Default|GetMaxBlackToWhiteTime))) :!class /Script/Engine.KismetMaterialLibrary)
        (Variables|Default|SetBlackToWhiteTime (- (Variables|Default|GetBlackToWhiteTime) (Utilities|Time|GetWorldDeltaSeconds)))
        (if (<= (Variables|Default|GetBlackToWhiteTime) 0.0)
          (Variables|Default|SetWhiteToBlackTime (Variables|Default|GetMaxWhiteToBlackTime))
          (Utilities|Array|RemoveItem (Utilities|Struct|BreakWeightedBlendables (Utilities|Struct|BreakPostProcessSettings (Variables|/Script/Engine.CameraComponent|GetPostProcessSettings (Variables|Default|GetPlayerCamera)))) (Utilities|Struct|MakeWeightedBlendable 1.0 (Variables|Default|GetEyeAdjustInst)))
          (Utilities|Array|Add (Utilities|Struct|BreakWeightedBlendables (Utilities|Struct|BreakPostProcessSettings (Variables|/Script/Engine.CameraComponent|GetPostProcessSettings (Variables|Default|GetPlayerCamera)))) (Utilities|Struct|MakeWeightedBlendable 1.0 (Variables|Default|GetHeadlightTransitionInst))))
        (elif (> (Variables|Default|GetWhiteToBlackTime) 0.0)
          (Rendering|Material|SetScalarParameterValue "/Game/Materials/MPC_EyeAdjust.MPC_EyeAdjust" "Intensity" (/ (Variables|Default|GetWhiteToBlackTime) (Variables|Default|GetMaxWhiteToBlackTime)) :!class /Script/Engine.KismetMaterialLibrary)
          (Variables|Default|SetWhiteToBlackTime (- (Variables|Default|GetWhiteToBlackTime) (Utilities|Time|GetWorldDeltaSeconds)))
          (if (<= (Variables|Default|GetWhiteToBlackTime) 0.0)
            (Variables|Default|SetTransitionTime (Variables|Default|GetMaxTransitionTime)))
          (else
            (Variables|Default|SetTransitionTime (- (Variables|Default|GetTransitionTime) (Utilities|Time|GetWorldDeltaSeconds)))
            (if (<= (Variables|Default|GetTransitionTime) 0.0)
              (Game|OpenLevel(byName) "Test"))))))))

(fn ConstructionScript)