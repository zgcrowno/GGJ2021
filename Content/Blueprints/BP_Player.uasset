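; BP_Player is a first-person player Character with mouse look, movement and highlighting of objects under the view.
; Every Tick, Move sets CharacterMovement velocity directly from input axes, MoveSpeed and delta time, preserving vertical velocity.
; Highlight then line-traces from the Camera up to InteractDistance, setting custom depth stencil 1 on hit components tagged "Highlightable" after resetting the previous one to 0.
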(event EventBeginPlay)

(event Collision|EventActorBeginOverlap
  (params (OtherActor :type Actor%20Object%20Reference)))

(event EventTick
  (params (DeltaSeconds :type Float%20%28single-precision%29))
  (CallFunction|Move)
  (CallFunction|Highlight))

(event Input|MouseEvents|MouseX
  (params (AxisValue :type Float%20%28single-precision%29))
  (Pawn|Input|AddControllerYawInput AxisValue))

(event Input|MouseEvents|MouseY
  (params (AxisValue :type Float%20%28single-precision%29))
  (bind _result (Math|Float|NegateFloat AxisValue)
    (:%20%20
      (Pawn|Input|AddControllerPitchInput _result))))

(fn ConstructionScript)

(fn Move
  (bind _returnvalue (Utilities|Time|GetWorldDeltaSeconds))
  (bind _movespeed (Variables|Default|GetMoveSpeed))
  (bind _output_get (LocalVariables|SetMovementVec (+ (+ (* (Transformation|GetActorForwardVector) (* (* (Input|AxisValues|GetMoveForward) _movespeed) _returnvalue)) (* (Transformation|GetActorRightVector) (* _returnvalue (* _movespeed (Input|AxisValues|GetMoveRight))))) (Math|Vector|MakeVector 0.0 0.0 (.Z (Math|Vector|BreakVector (Variables|/Script/Engine.MovementComponent|GetVelocity (Variables|Character|GetCharacterMovement))))))))
  (Variables|/Script/Engine.MovementComponent|SetVelocity (Variables|Character|GetCharacterMovement) _output_get))

(fn Highlight
  (bind _camera (Variables|Default|GetCamera))
  (bind _returnvalue (Transformation|GetWorldLocation _camera))
  (if (Utilities|IsValid (Variables|Default|GetHighlightedObject))
    (Rendering|SetCustomDepthStencilValue (Variables|Default|GetHighlightedObject) 0))
  (bind (_outhit _returnvalue_2) (Collision|LineTraceByChannel _returnvalue (+ _returnvalue (* (Math|Vector|GetForwardVector _camera) (Variables|Default|GetInteractDistance))) "TraceTypeQuery1" false 0 "None"))
  (if _returnvalue_2
    (if (Components|ComponentHasTag (.HitComponent (Collision|BreakHitResult _outhit)) "Highlightable")
      (bind _output_get (Variables|Default|SetHighlightedObject (.HitComponent (Collision|BreakHitResult _outhit))))
      (Rendering|SetCustomDepthStencilValue _output_get 1))))