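; First-person player pawn with interaction, a two-slot inventory for pickups and door keys, and movement-triggered ripples.
; Each Tick sets velocity from input, marks tagged components under a camera trace via custom depth stencil, and animates a ripple radius on a dynamic post-process material.
; Interact messages the first overlapping BPi_Interactable actor.
; Inventory functions fill free slots, report held key values, drop items ahead of the player, and destroy used keys.
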(event EventBeginPlay
  (Utilities|Array|AddUnique (Variables|Default|GetSenses) 0)
  (bind _returnvalue (Rendering|Material|CreateDynamicMaterialInstance "/Game/Materials/M_Highlight_Inst.M_Highlight_Inst" "None" :!class /Script/Engine.KismetMaterialLibrary))
  (bind _output_get (Variables|Default|SetRippleMaterialInst _returnvalue))
  (Utilities|Array|Add (Utilities|Struct|BreakWeightedBlendables (Utilities|Struct|BreakPostProcessSettings (Variables|/Script/Engine.CameraComponent|GetPostProcessSettings (Variables|Default|GetCamera)))) (Utilities|Struct|MakeWeightedBlendable 1.0 _output_get)))

(event Collision|EventActorBeginOverlap
  (params (OtherActor :type Actor%20Object%20Reference)))

(event EventTick
  (params (DeltaSeconds :type Float%20%28single-precision%29))
  (CallFunction|Move)
  (CallFunction|Highlight)
  (CallFunction|Ripple))

(event EventDestroyKey
  (params (Key%20to%20Destroy :type KeyEnum%20Enum :default "NewEnumerator3"))
  ;[1 1 1] Destroys the key and empties the inv slot (called when key is used by door)
  (if (Utilities|Enum|Equal(Enum) Key%20to%20Destroy (Variables|/Game/Blueprints/Environment/Item.Item_C|GetKeyValue (Variables|Default|GetInv_Slot_1)))
    (Actor|DestroyActor (Variables|Default|GetInv_Slot_1))
    (Variables|Default|SetInv_Slot_1 (Variables|Default|GetEmtpySlot))
    (elif (Utilities|Enum|Equal(Enum) Key%20to%20Destroy (Variables|/Game/Blueprints/Environment/Item.Item_C|GetKeyValue (Variables|Default|GetInv_Slot_2)))
      (Actor|DestroyActor (Variables|Default|GetInv_Slot_2))
      (Variables|Default|SetInv_Slot_2 (Variables|Default|GetEmtpySlot)))))

(event Input|ActionEvents|InputActionInteract
  (params (Key :type Key%20Structure))
  ;[1 1 1] Interact - Triggers "interaction" for first overlapping actor with interface
  (:Pressed
    (bind _array_element (Utilities|Array|ForEachLoopwithBreak (Collision|GetOverlappingActors (Variables|Collision|GetCapsuleComponent) 0 :!class /Script/Engine.PrimitiveComponent) :!label _label)
      (:LoopBody
        (if (Utilities|DoesObjectImplementInterface _array_element "/Game/Blueprints/BPi_Interactable.BPi_Interactable_C")
          (Class|BPiInteractable|Interaction(Message) _array_element self)
          (goto _label Break))))))

(event Input|ActionEvents|InputActionDropInvSlot2
  (params (Key :type Key%20Structure))
  ;[1 1 1] Drops item in slot2 into the world
  (:Pressed
    (if (!= (Variables|Default|GetInv_Slot_2) (Variables|Default|GetEmtpySlot))
      (Transformation|SetActorLocation (Variables|Default|GetInv_Slot_2) (+ (Transformation|GetWorldLocation (Variables|Collision|GetCapsuleComponent)) (* (Transformation|GetActorForwardVector) 75.0)) false false)
      (Variables|Default|SetInv_Slot_2 (Variables|Default|GetEmtpySlot)))))

(event Input|ActionEvents|InputActionDropInvSlot1
  (params (Key :type Key%20Structure))
  ;[1 1 1] Drops item in slot1 into the world
  (:Pressed
    (if (!= (Variables|Default|GetInv_Slot_1) (Variables|Default|GetEmtpySlot))
      (Transformation|SetActorLocation (Variables|Default|GetInv_Slot_1) (+ (Transformation|GetWorldLocation (Variables|Collision|GetCapsuleComponent)) (* (Transformation|GetActorForwardVector) 75.0)) false false)
      (Variables|Default|SetInv_Slot_1 (Variables|Default|GetEmtpySlot)))))

(event Input|MouseEvents|MouseX
  (params (AxisValue :type Float%20%28single-precision%29))
  (Pawn|Input|AddControllerYawInput AxisValue))

(event Input|MouseEvents|MouseY
  (params (AxisValue :type Float%20%28single-precision%29))
  (bind _result (Math|Float|NegateFloat AxisValue)
    (:%20%20
      (Pawn|Input|AddControllerPitchInput _result))))

(fn ConstructionScript)

(fn Move
  (bind _returnvalue (Utilities|Time|GetWorldDeltaSeconds))
  (bind _movespeed (Variables|Default|GetMoveSpeed))
  (bind _output_get (LocalVariables|SetMovementVec (+ (+ (* (Transformation|GetActorForwardVector) (* (* (Input|AxisValues|GetMoveForward) _movespeed) _returnvalue)) (* (Transformation|GetActorRightVector) (* _returnvalue (* _movespeed (Input|AxisValues|GetMoveRight))))) (Math|Vector|MakeVector 0.0 0.0 (.Z (Math|Vector|BreakVector (Variables|/Script/Engine.MovementComponent|GetVelocity (Variables|Character|GetCharacterMovement))))))))
  (bind _output_get_2 (Variables|/Script/Engine.MovementComponent|SetVelocity (Variables|Character|GetCharacterMovement) _output_get))
  (if (not (Math|Vector|Equal(Vector) _output_get_2 "0, 0, 0" 0.0001))
    (if (<= (Variables|Default|GetRippleLifetime) 0.0)
      (Variables|Default|SetRippleLifetime (Variables|Default|GetMaxRippleLifetime)))))

(fn Highlight
  (bind _camera (Variables|Default|GetCamera))
  (bind _returnvalue (Transformation|GetWorldLocation _camera))
  (if (Utilities|IsValid (Variables|Default|GetHighlightedObject))
    (Rendering|SetCustomDepthStencilValue (Variables|Default|GetHighlightedObject) 0))
  (bind (_outhit _returnvalue_2) (Collision|LineTraceByChannel _returnvalue (+ _returnvalue (* (Math|Vector|GetForwardVector _camera) (Variables|Default|GetInteractDistance))) "TraceTypeQuery1" false 0 "ForOneFrame"))
  (if _returnvalue_2
    (if (Components|ComponentHasTag (.HitComponent (Collision|BreakHitResult _outhit)) "Highlightable")
      (bind _output_get (Variables|Default|SetHighlightedObject (.HitComponent (Collision|BreakHitResult _outhit))))
      (Rendering|SetCustomDepthStencilValue _output_get 1))))

(fn Ripple
  (if (> (Variables|Default|GetRippleLifetime) 0.0)
    (Rendering|Material|SetScalarParameterValue 0 "Radius" (- 1.0 (/ (Variables|Default|GetRippleLifetime) (Variables|Default|GetMaxRippleLifetime))) :!class /Script/Engine.KismetMaterialLibrary)
    (Variables|Default|SetRippleLifetime (- (Variables|Default|GetRippleLifetime) (Utilities|Time|GetWorldDeltaSeconds)))))

(fn CheckforKey
  (bind _inv_slot_1 (Variables|Default|GetInv_Slot_1))
  (bind _inv_slot_2 (Variables|Default|GetInv_Slot_2))
  (if (!= (Variables|Default|GetEmtpySlot) _inv_slot_1)
    (Variables|Default|Setkv1 (Variables|/Game/Blueprints/Environment/Item.Item_C|GetKeyValue _inv_slot_1))
    (else
      (Variables|Default|Setkv1 (Variables|Default|GetNoneKey))))
  (if (!= _inv_slot_2 (Variables|Default|GetEmtpySlot))
    (Variables|Default|Setkv2 (Variables|/Game/Blueprints/Environment/Item.Item_C|GetKeyValue _inv_slot_2))
    (else
      (Variables|Default|Setkv2 (Variables|Default|GetNoneKey))))
  (return (Variables|Default|Getkv1) (Variables|Default|Getkv2)))

(fn PickUp
  (params (theItem :type Item%20Object%20Reference))
  (if (== (Variables|Default|GetInv_Slot_1) (Variables|Default|GetEmtpySlot))
    (Variables|Default|SetInv_Slot_1 theItem)
    (Development|PrintString "You picked up an item" :!label _label)
    (Variables|Default|SetpickedUp true)
    (elif (== (Variables|Default|GetInv_Slot_2) (Variables|Default|GetEmtpySlot))
      (Variables|Default|SetInv_Slot_2 theItem)
      (goto _label)
      (else
        (Development|PrintString "Your Hands are Full")
        (Variables|Default|SetpickedUp false))))
  (return (Variables|Default|GetpickedUp)))